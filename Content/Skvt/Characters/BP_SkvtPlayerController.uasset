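; Player controller for Skvt that sets up Enhanced Input, swaps the possessed character and toggles the main menu.
; BeginPlay adds the default, swap and camera mapping contexts and creates a HUD widget, whose storing and viewport step is disconnected.
; Swap possesses the next BP_SkvtBaseChar in the world, wrapping to the first.
; The menu toggle creates or removes WBP_MainMenu with the cursor, restoring game-only input on close.
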(event `self.ReceiveBeginPlay`
  (`self.InitializeInput`)
  (`self.ShowHUD`))

(event `EnhancedInput|/Game/Skvt/Characters/Input/Actions/IA_Swap`
  (params (ActionValue :type Boolean) (ElapsedSeconds :type "Float (double-precision)") (TriggeredSeconds :type "Float (double-precision)") (InputAction :type "InputAction Object Reference" :default "/Game/Skvt/Characters/Input/Actions/IA_Swap.IA_Swap"))
  (:`Triggered`
    (bind _outactors (`GameplayStatics.GetAllActorsOfClass` "/Game/Skvt/Characters/BP_SkvtBaseChar.BP_SkvtBaseChar_C"))
    (`self.Possess` (`self.FindNextCharacter` _outactors))))

(event `EnhancedInput|/Game/Skvt/Characters/Input/Actions/IA_ToggleOpenMenu`
  (params (ActionValue :type Boolean) (ElapsedSeconds :type "Float (double-precision)") (TriggeredSeconds :type "Float (double-precision)") (InputAction :type "InputAction Object Reference" :default "/Game/Skvt/Characters/Input/Actions/IA_ToggleOpenMenu.IA_ToggleOpenMenu"))
  (:`Triggered`
    (if (`self.IsMenuOpen`)
      (`self.CloseMenu`)
      (else
        (`self.OpenMenu`)))))

(fn `CloseMenu`
  (bind _mainmenuref (`self.MainMenuRef`))
  (`/Engine/EditorBlueprintResources/StandardMacros.IsValid` _mainmenuref
    (:`Is Valid`
      (`Widget.RemoveFromParent` _mainmenuref)
      (set `self.MainMenuRef` null)
      (set `self.bShowMouseCursor` false)
      (`WidgetBlueprintLibrary.SetInputMode_GameOnly` self)
      (`GameplayStatics.SetGamePaused` false))))

(fn `FindNextCharacter`
  (params (AvalibleCharacters :type "Array of Pawn Object Reference"))
  (returns (NextCharRef :type "Pawn Object Reference"))
  (locals (CharacterIndex :type Integer))
  (bind _avaliblecharacters (`local.AvalibleCharacters`))
  (bind _returnvalue (`KismetArrayLibrary.Array_Find` _avaliblecharacters (`self.K2_GetPawn`)))
  (bind _returnvalue_2 (+ (`local.CharacterIndex`) 1))
  (`|ExecutionSequence`
    (:`then_0`
      (if (`KismetArrayLibrary.Array_IsValidIndex` _avaliblecharacters _returnvalue)
        (set `local.CharacterIndex` _returnvalue)
        (else
          (return null))))
    (:`then_1`
      (if (`KismetArrayLibrary.Array_IsValidIndex` AvalibleCharacters _returnvalue_2)
        (return (`|GetArrayItem` (`local.AvalibleCharacters`) _returnvalue_2))
        (else
          (return (`|GetArrayItem` (`local.AvalibleCharacters`))))))))

(fn `InitializeInput`
  (bind _returnvalue (pcsubsystem `EnhancedInputLocalPlayerSubsystem` self))
  (`/Engine/EditorBlueprintResources/StandardMacros.IsValid` _returnvalue
    (:`Is Valid`
      (`EnhancedInputSubsystemInterface.AddMappingContext` _returnvalue "/Game/ThirdPerson/Input/IMC_Default.IMC_Default" 0 (struct))
      (`EnhancedInputSubsystemInterface.AddMappingContext` _returnvalue "/Game/Skvt/Characters/Input/IMC_SwapPawn.IMC_SwapPawn" 0 (struct))
      (`EnhancedInputSubsystemInterface.AddMappingContext` _returnvalue "/Game/Skvt/Characters/Input/IMC_Camera.IMC_Camera" 0 (struct)))))

(fn `IsMenuOpen`
  (returns (IsOpen :type Boolean))
  (`/Engine/EditorBlueprintResources/StandardMacros.IsValid` (`self.MainMenuRef`)
    (:`Is Valid`
      (return true))
    (:`Is Not Valid`
      (return false))))

(fn `OpenMenu`
  (bind _returnvalue (`|CreateWidget` "/Game/Skvt/UI/Widgets/Menu/WBP_MainMenu.WBP_MainMenu_C" self))
  (bind _output_get (set `self.MainMenuRef` _returnvalue))
  (`UserWidget.AddToViewport` _output_get 0)
  (set `self.bShowMouseCursor` true))

(fn `ShowHUD`
  (bind _returnvalue (`|CreateWidget` "/Game/Skvt/Characters/WBP_HUD.WBP_HUD_C" self)))

(fn `UserConstructionScript`)