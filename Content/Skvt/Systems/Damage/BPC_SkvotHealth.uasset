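; BPC_SkvotHealth is a component that tracks health and death for its owner.
; DealDamage ignores hits once dead, otherwise subtracts damage from Health, clamped between zero and MaxHealth.
; IsDead reports whether Health is exactly zero, and the OnDeath dispatcher fires on the hit that depletes it.
; The event graph holds no active logic, so changes happen only through calls.
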(fn `DealDamage`
  (params (Damage :type "Float (double-precision)"))
  (if (not (`self.IsDead`))
    (set `self.Health` (`KismetMathLibrary.FClamp` (- (`self.Health`) Damage) 0.0 (`self.MaxHealth`)))
    (if (`self.IsDead`)
      (`self.OnDeath`))))

(fn `IsDead`
  (returns (Dead :type Boolean))
  (return (== (`self.Health`) 0.0)))